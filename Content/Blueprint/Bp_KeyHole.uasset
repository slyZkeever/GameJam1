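; Keyhole puzzle that slides a door by an offset when a Bp_Key is socketed, and back when the key leaves.
; Box overlap snaps the key to HoleSocket, disables its physics, releases the player's Grabber, swaps materials and plays the DoorDriver timeline.
; End overlap undoes this and reverses the timeline.
; The begin check requires the overlapping actor to be the key-tagged player character, yet then casts it to Bp_Key.
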(event OnComponentBeginOverlap(Box)
  (params (OverlappedComponent :type Primitive%20Component%20Object%20Reference) (OtherActor :type Actor%20Object%20Reference) (OtherComp :type Primitive%20Component%20Object%20Reference) (OtherBodyIndex :type Integer) (bFromSweep :type Boolean) (SweepResult :type Hit%20Result%20Structure%20%28by%20ref%29))
  ;[1 1 1] On BeginOverlap
  (if (and (== (stale OnComponentBeginOverlap(PlayerCollision) OtherActor) (Game|GetPlayerCharacter 0)) (Actor|ActorHasTag OtherActor "key"))
    (Rendering|Material|SetMaterial (Variables|Default|GetHole) 0 "/Game/Materials/MatI_Interactable.MatI_Interactable")
    (bind _asbp_key (Utilities|Casting|CastToBp_Key OtherActor))
    (Physics|SetSimulatePhysics (Variables|/Game/Blueprint/Bp_Key.Bp_Key_C|GetKey _asbp_key) false)
    (Rendering|Material|SetMaterial (Variables|/Game/Blueprint/Bp_Key.Bp_Key_C|GetKey _asbp_key) 0 "/Game/Materials/MatI_HoleDeactive.MatI_HoleDeactive")
    (Transformation|AttachComponentToComponent (Variables|/Script/Engine.Actor|GetRootComponent _asbp_key) (Variables|Default|GetHole) "HoleSocket" "SnapToTarget" "SnapToTarget" "KeepWorld" true)
    (bind _asplayer_new (Utilities|Casting|CastToPlayer_New (Game|GetPlayerCharacter 0)))
    (Class|Grabber|SetGrabbed (Variables|/Game/Blueprint/Player_New.Player_New_C|GetGrabber _asplayer_new) false)
    (Class|Grabber|Drop (Variables|/Game/Blueprint/Player_New.Player_New_C|GetGrabber _asplayer_new))
    ;[1 1 1] Perform Animation
    (bind _newtrack_0 (Timeline|DoorDriver Play)
      (:Update
        (Transformation|SetRelativeLocation (Variables|Default|GetDoor) (Math|Vector|Lerp(Vector) (Variables|Default|GetDoorStartLocation) (Variables|Default|GetDoorEndLocation) _newtrack_0) false false)))))

(event OnComponentBeginOverlap(PlayerCollision)
  (params (OverlappedComponent :type Primitive%20Component%20Object%20Reference) (OtherActor :type Actor%20Object%20Reference) (OtherComp :type Primitive%20Component%20Object%20Reference) (OtherBodyIndex :type Integer) (bFromSweep :type Boolean) (SweepResult :type Hit%20Result%20Structure%20%28by%20ref%29))
  ;[1 1 1] Player Collision
)

(event OnComponentEndOverlap(Box)
  (params (OverlappedComponent :type Primitive%20Component%20Object%20Reference) (OtherActor :type Actor%20Object%20Reference) (OtherComp :type Primitive%20Component%20Object%20Reference) (OtherBodyIndex :type Integer))
  ;[1 1 1] On EndOverlap
  (bind _asbp_key (Utilities|Casting|CastToBp_Key OtherActor))
  (Physics|SetSimulatePhysics (Variables|/Game/Blueprint/Bp_Key.Bp_Key_C|GetKey _asbp_key) true)
  (Rendering|Material|SetMaterial (Variables|/Game/Blueprint/Bp_Key.Bp_Key_C|GetKey _asbp_key) 0 "/Game/Materials/MatI_Interactable.MatI_Interactable")
  (Transformation|DetachFromComponent (Variables|/Script/Engine.Actor|GetRootComponent _asbp_key) "KeepRelative" "KeepRelative" "KeepRelative" true)
  (Rendering|Material|SetMaterial (Variables|Default|GetHole) 0 "/Game/Materials/MatI_HoleDeactive.MatI_HoleDeactive")
  ;[1 1 1] Perform Animation
  (bind _newtrack_0 (Timeline|DoorDriver Reverse)
    (:Update
      (Transformation|SetRelativeLocation (Variables|Default|GetDoor) (Math|Vector|Lerp(Vector) (Variables|Default|GetDoorStartLocation) (Variables|Default|GetDoorEndLocation) _newtrack_0) false false))))

(event EventBeginPlay
  ;[1 1 1] Set Start and End Location of door
  (bind _output_get (Variables|Default|SetDoorStartLocation (.location (Transformation|GetRelativeTransform (Variables|Default|GetDoor)))))
  (Variables|Default|SetDoorEndLocation (+ _output_get (Variables|Default|GetHowMuchToMove))))

(fn ConstructionScript)