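; Interactable spawner button that, on the Interact input, spawns items through SpawnableManager using SpawnCollider and plays a button sound.
; PassTraced enables input only when the button is traced and Player_New overlaps PlayerCollider, otherwise disabling it.
; At the MaxItems cap, SpawnableManager deletes extra interactables before spawning.
; DestroySpecificActor is an empty event, with its manager destroy call left unconnected.
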(event OnComponentBeginOverlap(PlayerCollider)
  (params (OverlappedComponent :type Primitive%20Component%20Object%20Reference) (OtherActor :type Actor%20Object%20Reference) (OtherComp :type Primitive%20Component%20Object%20Reference) (OtherBodyIndex :type Integer) (bFromSweep :type Boolean) (SweepResult :type Hit%20Result%20Structure%20%28by%20ref%29))
  ;[1 1 1] Chk is player overlapping?
  (Utilities|Casting|CastToPlayer_New OtherActor)
  (Variables|Default|SetOverlapped? true))

(event OnComponentEndOverlap(PlayerCollider)
  (params (OverlappedComponent :type Primitive%20Component%20Object%20Reference) (OtherActor :type Actor%20Object%20Reference) (OtherComp :type Primitive%20Component%20Object%20Reference) (OtherBodyIndex :type Integer))
  ;[1 1 1] Chk is player overlapping?
  (Utilities|Casting|CastToPlayer_New OtherActor)
  (Variables|Default|SetOverlapped? false))

(event Custom|Destroy%20Specific%20Actor
  (params (ActorToDestroy :type Actor%20Object%20Reference))
  ;[1 1 1] Destroy specific actor
)

(event EventPassTraced
  (params (Traced? :type Boolean))
  ;[1 1 1] Enable/Disable Input
  (if (and Traced? (Variables|Default|GetOverlapped?))
    (Utilities|Casting|CastToPlayer_New (Game|GetPlayerCharacter 0))
    (Input|EnableInput (Game|GetPlayerController 0))
    (else
      (Utilities|Casting|CastToPlayer_New (Game|GetPlayerCharacter 0))
      (Input|DisableInput (Game|GetPlayerController 0)))))

(event Input|ActionEvents|InputActionInteract
  (params (Key :type Key%20Structure))
  (bind _spawnablemanager (Variables|Default|GetSpawnableManager))
  ;[1 1 1] Manage Cubes
  (:Pressed
    (Utilities|FlowControl|Sequence
      (:then_0
        (bind _returnvalue (Class|SpawnableManager|GetArrayLength (Variables|Default|GetSpawnableManager)))
        (if (< _returnvalue (Variables|Default|GetMaxItems))
          _
          (else
            (Class|SpawnableManager|DeleteExtraInteractables _spawnablemanager)))
        (Class|SpawnableManager|SpawnInteractables _spawnablemanager (Variables|Default|GetSpawnCollider)))
      (:then_1
        (Audio|PlaySoundatLocation "/Game/Sound/button_hit.button_hit" (Transformation|GetWorldLocation (Variables|Default|GetButton)))))))

(fn ConstructionScript)