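; Pressure plate Blueprint that tallies the mass of actors inside its Box component.
; On each begin overlap, it loops over all overlapping actors and adds the Mass of the player character or the physics mass of any BP_Interactable to TotalMass.
; The running total is printed, with no reset or end-overlap subtraction, so actors already inside are counted again on each new overlap.
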(event OnComponentBeginOverlap(Box)
  (params (OverlappedComponent :type Primitive%20Component%20Object%20Reference) (OtherActor :type Actor%20Object%20Reference) (OtherComp :type Primitive%20Component%20Object%20Reference) (OtherBodyIndex :type Integer) (bFromSweep :type Boolean) (SweepResult :type Hit%20Result%20Structure%20%28by%20ref%29))
  (for _array_element (Collision|GetOverlappingActors (Variables|Default|GetBox) "/Script/Engine.Actor" :!class /Script/Engine.PrimitiveComponent)
    (Utilities|FlowControl|Sequence
      (:then_0
        (if (== (Game|GetPlayerCharacter 0) _array_element)
          (bind _asplayer_new (Utilities|Casting|CastToPlayer_New _array_element))
          (Variables|Default|SetTotalMass (+ (Variables|/Game/Blueprint/Player_New.Player_New_C|GetMass _asplayer_new) (Variables|Default|GetTotalMass)))
          (Development|PrintString (Utilities|String|ToString(Float) (stale _output_get)) :!label _label)))
      (:then_1
        (if (== (Utilities|GetClass _array_element) "/Game/Blueprint/BP_Interactable.BP_Interactable_C")
          (bind _asbp_interactable (Utilities|Casting|CastToBP_Interactable _array_element))
          (bind _output_get (Variables|Default|SetTotalMass (+ (Physics|GetMass (Variables|/Script/Engine.StaticMeshActor|GetStaticMeshComponent _asbp_interactable)) (Variables|Default|GetTotalMass))))
          (goto _label))))))

(fn ConstructionScript)