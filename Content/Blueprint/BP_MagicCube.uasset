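; BP_MagicCube is a physics cube the player can grab, which sticks in place on overlapping an actor tagged Bp_Interactable.
; On overlap it stops simulating physics and makes the player's Grabber drop; the code to re-enable physics is disconnected.
; Hits play an impact sound, throttled by a DoOnce that resets after a delay.
; Helpers override mass and destroy the cube through its owning spawner, after calling the player's HoldDropObject.
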(event OnComponentEndOverlap(Collision)
  (params (OverlappedComponent :type Primitive%20Component%20Object%20Reference) (OtherActor :type Actor%20Object%20Reference) (OtherComp :type Primitive%20Component%20Object%20Reference) (OtherBodyIndex :type Integer)))

(event OnComponentBeginOverlap(Collision)
  (params (OverlappedComponent :type Primitive%20Component%20Object%20Reference) (OtherActor :type Actor%20Object%20Reference) (OtherComp :type Primitive%20Component%20Object%20Reference) (OtherBodyIndex :type Integer) (bFromSweep :type Boolean) (SweepResult :type Hit%20Result%20Structure%20%28by%20ref%29))
  ;[1 1 1] Stick interactables
  (if (Actor|ActorHasTag OtherActor "Bp_Interactable")
    (Physics|SetSimulatePhysics (Variables|Debug|GetStaticMeshComponent) false)
    (bind _asplayer_new (Utilities|Casting|CastToPlayer_New (Game|GetPlayerCharacter 0)))
    (Class|Grabber|Drop (Variables|/Game/Blueprint/Player_New.Player_New_C|GetGrabber _asplayer_new))
    (Utilities|FlowControl|Delay 1.0)))

(event OnComponentHit(StaticMeshComponent)
  (params (HitComponent :type Primitive%20Component%20Object%20Reference) (OtherActor :type Actor%20Object%20Reference) (OtherComp :type Primitive%20Component%20Object%20Reference) (NormalImpulse :type Vector :default "0, 0, 0") (Hit :type Hit%20Result%20Structure%20%28by%20ref%29))
  ;[1 1 1] Play Sound On Hit
  (Utilities|FlowControl|DoOnce false
    (:Completed
      (Audio|PlaySoundatLocation "/Game/Sound/object_hit.object_hit" (Transformation|GetWorldLocation HitComponent) "0, 0, 0" 1.0 1.0 0.0 0 0 0)
      (Utilities|FlowControl|Delay 1.0)
      (CallFunction|Reset))))

(event Custom|Reset
  ;[1 1 1] Play Sound On Hit
  (Utilities|FlowControl|DoOnce false) ; enters at Reset
)

(event EventBeginPlay)

(fn ConstructionScript)

(fn SetMass
  (params (MassToSet :type Float%20%28single-precision%29))
  (Class|PrimitiveComponent|SetMassOverrideinKg (Variables|Debug|GetStaticMeshComponent) "None" MassToSet true))

(fn Destroy
  (bind _asplayer_new (Utilities|Casting|CastToPlayer_New (Game|GetPlayerCharacter 0)))
  (Default|HoldDropObject _asplayer_new)
  (Utilities|IsValid (Variables|Default|GetOwningSpawnner)
    (:Is%20Valid
      (Default|DestroySpecificActor (Variables|Default|GetOwningSpawnner) self))
    (:Is%20Not%20Valid
      (Actor|DestroyActor))))