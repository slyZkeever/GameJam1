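; BP_Movers is a platform that travels between endpoints A and B, operated by the player's Interact input.
; Input is enabled only while PassTraced reports a trace and the player overlaps either end.
; Overlap volumes feed player and platform state to Movable, which handles timing, switching and animation, ticked only when recently rendered.
; Button, start and end sounds play, the latter two debounced by DoOnce with delayed resets.
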(event OnComponentEndOverlap(InteractWithPlatformAtB)
  (params (OverlappedComponent :type Primitive%20Component%20Object%20Reference) (OtherActor :type Actor%20Object%20Reference) (OtherComp :type Primitive%20Component%20Object%20Reference) (OtherBodyIndex :type Integer))
  ;[1 1 1] Platform Overlap
  (Utilities|FlowControl|DoOnce false
    (:Completed
      (Audio|PlaySoundatLocation "/Game/Sound/Elevator/start.start" (Transformation|GetWorldLocation (Variables|Default|GetPlatform)))
      (Utilities|FlowControl|Delay 1.0)
      (CallFunction|Reset1))))

(event OnComponentEndOverlap(InteractWithPlatformAtA)
  (params (OverlappedComponent :type Primitive%20Component%20Object%20Reference) (OtherActor :type Actor%20Object%20Reference) (OtherComp :type Primitive%20Component%20Object%20Reference) (OtherBodyIndex :type Integer))
  ;[1 1 1] Platform Overlap
  (Utilities|FlowControl|DoOnce false
    (:Completed
      (Audio|PlaySoundatLocation "/Game/Sound/Elevator/start.start" (Transformation|GetWorldLocation (Variables|Default|GetPlatform)))
      (Utilities|FlowControl|Delay 1.0)
      (CallFunction|Reset1))))

(event OnComponentBeginOverlap(InteractWithPlatformAtA)
  (params (OverlappedComponent :type Primitive%20Component%20Object%20Reference) (OtherActor :type Actor%20Object%20Reference) (OtherComp :type Primitive%20Component%20Object%20Reference) (OtherBodyIndex :type Integer) (bFromSweep :type Boolean) (SweepResult :type Hit%20Result%20Structure%20%28by%20ref%29))
  ;[1 1 1] Platform Overlap
  (if (== OtherComp (Variables|Default|GetPlatform))
    (Class|Movable|SetPlatformatA (Variables|Default|GetMovable) true)
    (Utilities|FlowControl|DoOnce false
      (:Completed
        (Audio|PlaySoundatLocation "/Game/Sound/Elevator/end.end" (Transformation|GetWorldLocation (Variables|Default|GetPlatform)))
        (Utilities|FlowControl|Delay 1.0)
        (CallFunction|Reset)))))

(event OnComponentBeginOverlap(InteractWithPlatformAtB)
  (params (OverlappedComponent :type Primitive%20Component%20Object%20Reference) (OtherActor :type Actor%20Object%20Reference) (OtherComp :type Primitive%20Component%20Object%20Reference) (OtherBodyIndex :type Integer) (bFromSweep :type Boolean) (SweepResult :type Hit%20Result%20Structure%20%28by%20ref%29))
  ;[1 1 1] Platform Overlap
  (if (== (Variables|Default|GetPlatform) OtherComp)
    (Class|Movable|SetPlatformatA (Variables|Default|GetMovable) false)
    (Utilities|FlowControl|DoOnce false
      (:Completed
        (Audio|PlaySoundatLocation "/Game/Sound/Elevator/end.end" (Transformation|GetWorldLocation (Variables|Default|GetPlatform)))
        (Utilities|FlowControl|Delay 1.0)
        (CallFunction|Reset)))))

(event OnComponentBeginOverlap(InteractWithPlayerAtB)
  (params (OverlappedComponent :type Primitive%20Component%20Object%20Reference) (OtherActor :type Actor%20Object%20Reference) (OtherComp :type Primitive%20Component%20Object%20Reference) (OtherBodyIndex :type Integer) (bFromSweep :type Boolean) (SweepResult :type Hit%20Result%20Structure%20%28by%20ref%29))
  ;[1 1 1] Get Player Overlap
  (Utilities|Casting|CastToPlayer_New OtherActor)
  (Class|Movable|SetPlayeratB (Variables|Default|GetMovable) true))

(event OnComponentEndOverlap(InteractWithPlayerAtB)
  (params (OverlappedComponent :type Primitive%20Component%20Object%20Reference) (OtherActor :type Actor%20Object%20Reference) (OtherComp :type Primitive%20Component%20Object%20Reference) (OtherBodyIndex :type Integer))
  ;[1 1 1] Get Player Overlap
  (Class|Movable|SetPlayeratB (Variables|Default|GetMovable) false))

(event OnComponentEndOverlap(InteractWithPlayerAtA)
  (params (OverlappedComponent :type Primitive%20Component%20Object%20Reference) (OtherActor :type Actor%20Object%20Reference) (OtherComp :type Primitive%20Component%20Object%20Reference) (OtherBodyIndex :type Integer))
  ;[1 1 1] Get Player Overlap
  (Class|Movable|SetPlayeratA (Variables|Default|GetMovable) false))

(event OnComponentBeginOverlap(InteractWithPlayerAtA)
  (params (OverlappedComponent :type Primitive%20Component%20Object%20Reference) (OtherActor :type Actor%20Object%20Reference) (OtherComp :type Primitive%20Component%20Object%20Reference) (OtherBodyIndex :type Integer) (bFromSweep :type Boolean) (SweepResult :type Hit%20Result%20Structure%20%28by%20ref%29))
  ;[1 1 1] Get Player Overlap
  (Utilities|Casting|CastToPlayer_New OtherActor)
  (Class|Movable|SetPlayeratA (Variables|Default|GetMovable) true))

(event Custom|Reset
  ;[1 1 1] Platform Overlap
  (Utilities|FlowControl|DoOnce false) ; enters at Reset
)

(event Custom|Reset1
  ;[1 1 1] Platform Overlap
  (Utilities|FlowControl|DoOnce false) ; enters at Reset
)

(event Custom|Chk%20Player%20Overlap
  (bind _movable (Variables|Default|GetMovable))
  ;[1 1 1] Enable/Disable Input
  (bind _returnvalue (Class|Movable|GetPlayeratA _movable))
  (bind _returnvalue_2 (Class|Movable|GetPlayeratB _movable)))

(event EventPassTraced
  (params (Traced? :type Boolean))
  ;[1 1 1] Enable/Disable Input
  (CallFunction|ChkPlayerOverlap)
  (if (and Traced? (or (stale Custom|Chk%20Player%20Overlap _returnvalue) (stale Custom|Chk%20Player%20Overlap _returnvalue_2)))
    (Input|EnableInput (Game|GetPlayerController 0))
    (Class|Movable|CalculateTime (Variables|Default|GetMovable) (Variables|Default|GetInteractWithPlatformAtA) (Variables|Default|GetInteractWithPlatformAtB))
    (else
      (Input|DisableInput (Game|GetPlayerController 0)))))

(event EventTick
  (params (DeltaSeconds :type Float%20%28single-precision%29))
  ;[1 1 1] Perform Animation
  (if (Class|Actor|WasRecentlyRendered 0.2)
    (Class|Movable|PerformAnimation (Variables|Default|GetMovable) (Variables|Default|GetPlatform))))

(event Input|ActionEvents|InputActionInteract
  (params (Key :type Key%20Structure))
  ;[1 1 1] Manage Input
  (:Pressed
    (Audio|PlaySoundatLocation "/Game/Sound/button_hit.button_hit" (Transformation|GetWorldLocation (Variables|Default|GetInteractWithPlayerAtA)))
    (Class|Movable|Switcher (Variables|Default|GetMovable))))

(fn ConstructionScript)